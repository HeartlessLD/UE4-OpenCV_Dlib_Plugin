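; Webcam actor that shows the camera feed on a mesh and drives a simple face puppet from face-tracking data.
; On Android it polls for camera permission before starting capture; other platforms start at BeginPlay, and each video frame feeds a dynamic material texture.
; Each tick, FaceThread's eye and mouth weights are clamped and remapped to scale the eye and mouth components, and its head rotator rotates the Head.
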(event `CheckPermission`
  ;[1 1 1] android 检测相机权限
  (bind _returnvalue (`AndroidPermissionFunctionLibrary.CheckPermission` "android.permission.CAMERA"))
  (if _returnvalue
    (`KismetSystemLibrary.K2_ClearTimer` null "CheckPermission")
    (`|ExecutionSequence` :!label _label
      (:`then_1`
        (`self.BeginCapture`)))))

(event `self.ReceiveBeginPlay`
  (switch `string` (`GameplayStatics.GetPlatformName`)
    (:`Default`
      (goto _label))
    (:`Android`
      ;[1 1 1] android 检测相机权限
      (`KismetSystemLibrary.K2_SetTimerDelegate` (delegate `CheckPermission`) 0.5 true))))

(event `self.OnNextVideoFrame`
  (`MaterialInstanceDynamic.SetTextureParameterValue` (`self.MeshMat`) "Tex" (`self.VideoTexture`)))

(event `self.ReceiveTick`
  (params (DeltaSeconds :type "Float (single-precision)"))
  (bind (_headrotator_roll _headrotator_pitch _headrotator_yaw) (`KismetMathLibrary.BreakRotator` (`FaceFrameCalcThread.HeadRotator` (`self.FaceThread`))))
  (`|ExecutionSequence`
    (:`then_0`
      (`SceneComponent.SetWorldScale3D` (`self.LeftEye`) (`KismetMathLibrary.VLerp` (0.1 0.1 0.1) (0.3 0.3 0.3) (/ (- (`KismetMathLibrary.FClamp` (`FaceFrameCalcThread.LeftEyeWeight` (`self.FaceThread`)) 0.4 0.6) 0.4) (- 0.6 0.4)))))
    (:`then_1`
      (`SceneComponent.SetWorldScale3D` (`self.RightEye`) (`KismetMathLibrary.VLerp` (0.1 0.1 0.1) (0.3 0.3 0.3) (/ (- (`KismetMathLibrary.FClamp` (`FaceFrameCalcThread.RightEyeWeight` (`self.FaceThread`)) 0.4 0.6) 0.4) (- 0.6 0.4)))))
    (:`then_2`
      (`SceneComponent.SetWorldScale3D` (`self.Mouse`) (`KismetMathLibrary.VLerp` (0.2 0.4 0.05) (0.2 0.4 0.3) (/ (- (`KismetMathLibrary.FClamp` (`FaceFrameCalcThread.MouseWeight` (`self.FaceThread`)) 0.05 0.2) 0.05) (- 0.2 0.05)))))
    (:`then_3`
      (`SceneComponent.K2_SetRelativeRotation` (`self.Head`) (`KismetMathLibrary.MakeRotator` _headrotator_roll _headrotator_pitch _headrotator_yaw) false false))))

(fn `UserConstructionScript`
  (bind _returnvalue (`PrimitiveComponent.CreateDynamicMaterialInstance` (`self.StaticMesh`) 0 "/Game/TestPlugin/M_WebMaterial.M_WebMaterial" "None"))
  (set `self.MeshMat` _returnvalue)
  (`PrimitiveComponent.SetMaterial` (`self.StaticMesh`) 0 _returnvalue))