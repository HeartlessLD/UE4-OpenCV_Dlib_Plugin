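; BP_Webcam is a test plugin actor that shows captured video, apparently from a webcam, on its static mesh.
; The construction script creates a dynamic instance of M_WebMaterial and assigns it to the mesh.
; BeginPlay starts capture after a short delay, and each OnNextVideoFrame event pushes VideoTexture into the material's Tex parameter.
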(event `self.ReceiveBeginPlay`
  (`KismetSystemLibrary.Delay` 5.0)
  (`self.BeginCapture`))

(event `self.OnNextVideoFrame`
  (`MaterialInstanceDynamic.SetTextureParameterValue` (`self.MeshMat`) "Tex" (`self.VideoTexture`)))

(fn `UserConstructionScript`
  (bind _returnvalue (`PrimitiveComponent.CreateDynamicMaterialInstance` (`self.StaticMesh`) 0 "/Game/TestPlugin/M_WebMaterial.M_WebMaterial" "None"))
  (set `self.MeshMat` _returnvalue)
  (`PrimitiveComponent.SetMaterial` (`self.StaticMesh`) 0 _returnvalue))